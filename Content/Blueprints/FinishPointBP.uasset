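; Level finish marker that bobs up and down and ends the level when touched.
; Any overlap with its Sphere prints a win message and opens the 2DSideScrollerExampleMap level, without checking which actor entered.
; From BeginPlay, MoveVertically loops endlessly, chaining eased MoveComponentTo calls on the root that alternate up and down.
; The Move helper derives each target by offsetting the root's relative Z by MovingDistance.
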(event OnComponentBeginOverlap(Sphere)
  (params (OverlappedComponent :type Primitive%20Component%20Object%20Reference) (OtherActor :type Actor%20Object%20Reference) (OtherComp :type Primitive%20Component%20Object%20Reference) (OtherBodyIndex :type Integer) (bFromSweep :type Boolean) (SweepResult :type Hit%20Result%20Structure%20%28by%20ref%29))
  (Development|PrintString "You Win")
  (Game|OpenLevel(byObjectReference) "/Game/Maps/2DSideScrollerExampleMap.2DSideScrollerExampleMap"))

(event EventBeginPlay
  (|MoveVertically))

(fn ConstructionScript)

(fn Move
  (params (DistanceToMove :type Float%20%28single-precision%29))
  (bind _defaultsceneroot (Variables|Default|GetDefaultSceneRoot))
  (bind _relativelocation (Variables|/Script/Engine.SceneComponent|GetRelativeLocation _defaultsceneroot))
  (bind (_x _y _z) (Math|Vector|BreakVector _relativelocation))
  (return (Math|Vector|MakeVector _x _y (- _z DistanceToMove))))