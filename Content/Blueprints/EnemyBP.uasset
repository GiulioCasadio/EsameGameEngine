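; Side-scroller enemy that patrols back and forth along X, kills the player on contact and can itself be destroyed.
; BeginPlay loops two eased MoveComponentTo calls on the root, with targets offset by MovingDistance through the Move helper.
; DamageArea overlap calls the player character's restart after a debug print, while overlap on either cone destroys the enemy without checking what touched it.
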(event OnComponentBeginOverlap(DamageArea)
  (params (OverlappedComponent :type Primitive%20Component%20Object%20Reference) (OtherActor :type Actor%20Object%20Reference) (OtherComp :type Primitive%20Component%20Object%20Reference) (OtherBodyIndex :type Integer) (bFromSweep :type Boolean) (SweepResult :type Hit%20Result%20Structure%20%28by%20ref%29))
  (Development|PrintString "Killed by enemy" true true "(R=1.000000,G=0.000000,B=0.134241,A=1.000000)")
  (bind _as2dside_scroller_character (Utilities|Casting|CastTo2DSideScrollerCharacter OtherActor))
  (Default|CallRestartPlayer _as2dside_scroller_character))

(event OnComponentBeginOverlap(Cone)
  (params (OverlappedComponent :type Primitive%20Component%20Object%20Reference) (OtherActor :type Actor%20Object%20Reference) (OtherComp :type Primitive%20Component%20Object%20Reference) (OtherBodyIndex :type Integer) (bFromSweep :type Boolean) (SweepResult :type Hit%20Result%20Structure%20%28by%20ref%29))
  (Actor|DestroyActor))

(event OnComponentBeginOverlap(Cone1)
  (params (OverlappedComponent :type Primitive%20Component%20Object%20Reference) (OtherActor :type Actor%20Object%20Reference) (OtherComp :type Primitive%20Component%20Object%20Reference) (OtherBodyIndex :type Integer) (bFromSweep :type Boolean) (SweepResult :type Hit%20Result%20Structure%20%28by%20ref%29))
  (Actor|DestroyActor))

(event EventBeginPlay
  (bind _defaultsceneroot (Variables|Default|GetDefaultSceneRoot))
  (bind _relativerotation (Variables|/Script/Engine.SceneComponent|GetRelativeRotation _defaultsceneroot))
  (bind _positiontomove (CallFunction|Move (* (Variables|Default|GetmovingDistance) -1.0) :!label _label))
  (Components|MoveComponentTo _defaultsceneroot _positiontomove _relativerotation true true 1.5 false)
  (bind _positiontomove_2 (CallFunction|Move (Variables|Default|GetmovingDistance)))
  (Components|MoveComponentTo _defaultsceneroot _positiontomove_2 _relativerotation true true 1.5 false)
  (goto _label))

(fn ConstructionScript)

(fn Move
  (params (distanceToMove :type Float%20%28single-precision%29))
  (bind _defaultsceneroot (Variables|Default|GetDefaultSceneRoot))
  (bind _relativelocation (Variables|/Script/Engine.SceneComponent|GetRelativeLocation _defaultsceneroot))
  (bind (_x _y _z) (Math|Vector|BreakVector _relativelocation))
  (return (Math|Vector|MakeVector (- _x distanceToMove) _y _z)))