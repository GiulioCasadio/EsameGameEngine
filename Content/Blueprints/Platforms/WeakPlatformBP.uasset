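; WeakPlatformBP is a side-scroller platform that gives way shortly after the character touches it.
; WeakCollision overlap with the character dims the sprite and starts a timer that makes PlatformSolid ignore collision and fade further.
; Ending that overlap restores blocking and full opacity and clears the timer.
; A separate CollisionTrigger makes the platform non-blocking while overlapped, with an IsBlocking flag guarding both toggles.
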(event OnComponentBeginOverlap(CollisionTrigger)
  (params (OverlappedComponent :type Primitive%20Component%20Object%20Reference) (OtherActor :type Actor%20Object%20Reference) (OtherComp :type Primitive%20Component%20Object%20Reference) (OtherBodyIndex :type Integer) (bFromSweep :type Boolean) (SweepResult :type Hit%20Result%20Structure%20%28by%20ref%29))
  (CallFunction|MakeNotCollildable (Variables|Default|GetPlatformSolid)))

(event OnComponentEndOverlap(CollisionTrigger)
  (params (OverlappedComponent :type Primitive%20Component%20Object%20Reference) (OtherActor :type Actor%20Object%20Reference) (OtherComp :type Primitive%20Component%20Object%20Reference) (OtherBodyIndex :type Integer))
  (CallFunction|MakeCollildable (Variables|Default|GetPlatformSolid)))

(event OnComponentBeginOverlap(WeakCollision)
  (params (OverlappedComponent :type Primitive%20Component%20Object%20Reference) (OtherActor :type Actor%20Object%20Reference) (OtherComp :type Primitive%20Component%20Object%20Reference) (OtherBodyIndex :type Integer) (bFromSweep :type Boolean) (SweepResult :type Hit%20Result%20Structure%20%28by%20ref%29))
  (Utilities|Casting|CastTo2DSideScrollerCharacter OtherActor)
  (bind _returnvalue (Utilities|Time|SetTimerbyEvent (delegate Custom|RemoveCollision) 2.0))
  (CallFunction|SetSpriteAlpha 0.6))

(event OnComponentEndOverlap(WeakCollision)
  (params (OverlappedComponent :type Primitive%20Component%20Object%20Reference) (OtherActor :type Actor%20Object%20Reference) (OtherComp :type Primitive%20Component%20Object%20Reference) (OtherBodyIndex :type Integer))
  (CallFunction|MakeCollildable (Variables|Default|GetPlatformSolid))
  (CallFunction|SetSpriteAlpha 1.0)
  (Utilities|Time|ClearandInvalidateTimerbyHandle (stale OnComponentBeginOverlap(WeakCollision) _returnvalue)))

(event Custom|AddCollision
  (CallFunction|MakeCollildable (Variables|Default|GetPlatformSolid))
  (CallFunction|SetSpriteAlpha 1.0)
  (Utilities|Time|ClearandInvalidateTimerbyHandle (stale OnComponentBeginOverlap(WeakCollision) _returnvalue)))

(event Custom|RemoveCollision
  (CallFunction|MakeNotCollildable (Variables|Default|GetPlatformSolid))
  (CallFunction|SetSpriteAlpha 0.2))

(fn ConstructionScript)

(fn MakeNotCollildable
  (params (self2 :type Primitive%20Component%20Object%20Reference))
  (if (Variables|Default|GetIsBlocking)
    (Collision|SetCollisionResponsetoAllChannels self2 "ECR_Ignore")
    (Variables|Default|SetIsBlocking false)))

(fn MakeCollildable
  (params (self2 :type Primitive%20Component%20Object%20Reference))
  (if (not (Variables|Default|GetIsBlocking))
    (Collision|SetCollisionResponsetoAllChannels self2 "ECR_Block")
    (Variables|Default|SetIsBlocking true)))

(fn SetSpriteAlpha
  (params (Alpha :type Float%20%28single-precision%29))
  (bind _platformsolid (Variables|Default|GetPlatformSolid))
  (bind _spritecolor (Variables|/Script/Paper2D.PaperSpriteComponent|GetSpriteColor _platformsolid))
  (bind (_r _g _b) (Math|Color|BreakColor _spritecolor))
  (Sprite|SetSpriteColor _platformsolid (Math|Color|MakeColor _r _g _b Alpha)))