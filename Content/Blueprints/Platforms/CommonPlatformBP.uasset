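; Platform Blueprint whose solid part turns passable while something overlaps its trigger volume.
; Begin overlap on CollisionTrigger sets PlatformSolid to ignore all collision channels, and end overlap restores blocking on all channels.
; An IsBlocking flag skips redundant switches.
; Overlaps are neither filtered by actor nor counted, so any single exit makes the platform solid again.
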(event OnComponentBeginOverlap(CollisionTrigger)
  (params (OverlappedComponent :type Primitive%20Component%20Object%20Reference) (OtherActor :type Actor%20Object%20Reference) (OtherComp :type Primitive%20Component%20Object%20Reference) (OtherBodyIndex :type Integer) (bFromSweep :type Boolean) (SweepResult :type Hit%20Result%20Structure%20%28by%20ref%29))
  (CallFunction|MakeNotCollildable (Variables|Default|GetPlatformSolid)))

(event OnComponentEndOverlap(CollisionTrigger)
  (params (OverlappedComponent :type Primitive%20Component%20Object%20Reference) (OtherActor :type Actor%20Object%20Reference) (OtherComp :type Primitive%20Component%20Object%20Reference) (OtherBodyIndex :type Integer))
  (CallFunction|MakeCollildable (Variables|Default|GetPlatformSolid)))

(fn ConstructionScript)

(fn MakeNotCollildable
  (params (self2 :type Primitive%20Component%20Object%20Reference))
  (if (Variables|Default|GetIsBlocking)
    (Collision|SetCollisionResponsetoAllChannels self2 "ECR_Ignore")
    (Variables|Default|SetIsBlocking false)))

(fn MakeCollildable
  (params (self2 :type Primitive%20Component%20Object%20Reference))
  (if (not (Variables|Default|GetIsBlocking))
    (Collision|SetCollisionResponsetoAllChannels self2 "ECR_Block")
    (Variables|Default|SetIsBlocking true)))